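; A VR button actor that returns the interacting player to the main menu.
; On a button state change it passes the state to its electrical targets as a current provider and swaps the on/off text.
; If the interactor's controller is a VRMainMenuPlayerController, it snaps the button off without re-firing the event.
; It then calls that controller's return-to-menu function directly on the server, or its server-call variant otherwise.
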(event OnButtonStateChanged(ButtonComp)
  (params (ButtonState :type Boolean) (InteractingActor :type Actor%20Object%20Reference) (InteractingComponent :type Primitive%20Component%20Object%20Reference))
  (bind _textrender (Variables|Default|GetTextRender))
  ;[1 1 1] Send Out Electrical Signal
  (for _array_element (Variables|Default|GetElectricalTargets)
    (bind _aselectrical_object (Utilities|Casting|CastToElectricalObject _array_element))
    (Default|CurrentStateChange _aselectrical_object self ButtonState 1.0))
  (if ButtonState
    (Rendering|Components|TextRender|SetText _textrender (Variables|Default|GetOnText))
    (else
      (Rendering|Components|TextRender|SetText _textrender (Variables|Default|GetOffText))))
  (bind _as폰 (Utilities|Casting|CastToPawn InteractingActor))
  (bind _asvrmain_menu_player_controller (Utilities|Casting|CastToVRMainMenuPlayerController (Pawn|GetController _as폰)))
  (Class|VRButtonComponent|SetButtonState (Variables|Default|GetButtonComp) false false true)
  (if (Networking|IsServer)
    (Default|ReturntoMainMenu _asvrmain_menu_player_controller)
    (else
      (Default|ReturntoMainMenuServerCall _asvrmain_menu_player_controller))))

(event EventBeginPlay
  (|CallParentFunction) ; 지금 이 노드는 비활성 상태입니다. \n핀을 끌어서 다른 노드를 연결하면 활성화됩니다.
)

(event Collision|EventActorBeginOverlap
  (params (OtherActor :type Actor%20Object%20Reference)))

(event EventTick
  (params (DeltaSeconds :type Float%20%28single-precision%29))
  (|CallParentFunction DeltaSeconds) ; 지금 이 노드는 비활성 상태입니다. \n핀을 끌어서 다른 노드를 연결하면 활성화됩니다.
)

(fn ConstructionScript
  (|CallParentFunction))