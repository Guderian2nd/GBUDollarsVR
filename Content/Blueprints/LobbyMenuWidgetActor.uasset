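; Actor that displays the VR lobby menu on a widget component, showing connected players, their ready status and the ready sequence.
; On BeginPlay it caches the LobbyMenuWidget, creating one on clients if missing; the server also binds to VRMainMenuGameMode's dispatchers.
; Those dispatchers drive wrapper events that rebuild the name list or start and abort the ready sequence.
; List updates wait tick by tick until the widget is valid.
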(event Custom|ClearAndUpdatePlayerNamesAll
  (params (PlayerProfiles :type Array%20of%20S%20Player%20Profile%20Structures) (AllPlayerREadyStatus :type Array%20of%20Booleans))
  (bind _lobbymenuumg (Variables|Default|GetLobbyMenuUMG))
  (Utilities|IsValid _lobbymenuumg
    (:Is%20Valid
      _)
    (:Is%20Not%20Valid
      (CallFunction|InitLobbyMenuUMG)
      (if (Utilities|IsValid _lobbymenuumg) :!label _label
        _
        (else
          (Utilities|FlowControl|DelayUntilNextTick)
          (goto _label)))))
  (Default|ClearPlayerNames _lobbymenuumg)
  (Default|UpdatePlayerNames _lobbymenuumg PlayerProfiles AllPlayerREadyStatus))

(event Custom|ConnectedPlayerListChanged
  (CallFunction|ClearandUpdatePlayerNamesAll (Variables|/Game/Blueprints/VRMainMenuGameMode.VRMainMenuGameMode_C|GetAllPlayerProfiles (stale EventBeginPlay _asvrmain_menu_game_mode)) (Variables|/Game/Blueprints/VRMainMenuGameMode.VRMainMenuGameMode_C|GetAllPlayersReadyStatus (stale EventBeginPlay _asvrmain_menu_game_mode))))

(event Custom|CallStartReadySequence
  (CallFunction|ServerStartReadySequence))

(event Custom|CallAbortReadySequence
  (CallFunction|ServerAbortReadySequence))

(event Custom|ServerStartReadySequence
  (Default|StartReadySequence (Variables|Default|GetLobbyMenuUMG)))

(event Custom|ServerAbortReadySequence
  (Default|AbortReadySequence (Variables|Default|GetLobbyMenuUMG)))

(event EventBeginPlay
  (bind _lobbymenuumg (Variables|Default|GetLobbyMenuUMG))
  (CallFunction|InitLobbyMenuUMG)
  (if (Networking|IsServer)
    (bind _asvrmain_menu_game_mode (Utilities|Casting|CastToVRMainMenuGameMode (Game|GetGameMode)))
    (CallFunction|BindEventDispatchers _asvrmain_menu_game_mode (delegate Custom|ConnectedPlayerListChanged) (delegate Custom|CallStartReadySequence) (delegate Custom|CallAbortReadySequence))
    (Default|ClearPlayerNames _lobbymenuumg)
    (Default|UpdatePlayerNames _lobbymenuumg (Variables|/Game/Blueprints/VRMainMenuGameMode.VRMainMenuGameMode_C|GetAllPlayerProfiles _asvrmain_menu_game_mode) (Variables|/Game/Blueprints/VRMainMenuGameMode.VRMainMenuGameMode_C|GetAllPlayersReadyStatus _asvrmain_menu_game_mode))))

(event Collision|EventActorBeginOverlap
  (params (OtherActor :type Actor%20Object%20Reference)))

(event EventTick
  (params (DeltaSeconds :type Float%20%28single-precision%29)))

(fn ConstructionScript)

(fn InitLobbyMenuUMG
  (bind _widget (Variables|Default|GetWidget))
  (bind _returnvalue (UserInterface|GetWidget _widget))
  (Utilities|IsValid _returnvalue
    (:Is%20Valid
      (bind _aslobby_menu_widget (Utilities|Casting|CastToLobbyMenuWidget _returnvalue))
      (bind _output_get (Variables|Default|SetLobbyMenuUMG _aslobby_menu_widget))
      (return _output_get))
    (:Is%20Not%20Valid
      (if (not (Networking|IsServer))
        (bind _returnvalue_2 (UserInterface|CreateWidget "/Game/Blueprints/UMGs/LobbyMenuWidget.LobbyMenuWidget_C" (Game|GetPlayerController 0)))
        (UserInterface|SetWidget _widget _returnvalue_2)
        (bind _output_get_2 (Variables|Default|SetLobbyMenuUMG _returnvalue_2))
        (return _output_get_2)))))

(fn BindEventDispatchers
  (params (VRMainMenuGameMode :type VR%20Main%20Menu%20Game%20Mode%20Object%20Reference) (ConnectedPlayerListChanged :type Delegate%20%28by%20ref%29) (CallStartReadySequence :type Delegate%20%28by%20ref%29) (CallAbortReadySequence :type Delegate%20%28by%20ref%29))
  (EventDispatchers|BindEventtoConnectedPlayerListChanged VRMainMenuGameMode ConnectedPlayerListChanged)
  (EventDispatchers|BindEventtoStartReadySequence VRMainMenuGameMode CallStartReadySequence)
  (EventDispatchers|BindEventtoAbortReadySequence VRMainMenuGameMode CallAbortReadySequence))