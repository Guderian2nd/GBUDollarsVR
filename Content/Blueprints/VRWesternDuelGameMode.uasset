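; Game mode for a three-player VR Western duel that tracks connected controllers and occupied player starts.
; On the Duel Map, joining players are registered and run entry setup next tick.
; The third join triggers a countdown on every controller, flagging one random player as Iron Man.
; Logout frees that player's start; helpers split starts by occupied tag and find the "Host" start.
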(event Custom|AllPlayersConnected
  (Utilities|FlowControl|Delay 0.2)
  (bind _output_get (Variables|Default|SetIronManIndex (Math|Random|RandomIntegerinRange 0 2)))
  (for (_array_element _array_index) (Variables|Default|GetAllConnectedPlayers)
    (Default|GameStartCountDown _array_element (== _array_index _output_get))))

(event EventBeginPlay)

(event EventTick
  (params (DeltaSeconds :type Float%20%28single-precision%29)))

(event EventSetPlayerStartOccupied
  (params (OccupyingPlayer :type VR%20Western%20Player%20Controller%20Base%20Object%20Reference) (OccupyingPosition :type String))
  (bind _asvrwestern_player_controller (Utilities|Casting|CastToVRWesternPlayerController OccupyingPlayer))
  (Utilities|Map|Add (Variables|Default|GetOccupiedPlayerStarts) OccupyingPosition _asvrwestern_player_controller))

(event EventOnLogout
  (params (ExitingController :type Controller%20Object%20Reference))
  (bind _asvrwestern_player_controller (Utilities|Casting|CastToVRWesternPlayerController ExitingController))
  (Utilities|Array|RemoveItem (Variables|Default|GetAllConnectedPlayers) _asvrwestern_player_controller)
  (CallFunction|FindandFreePlayerStart _asvrwestern_player_controller))

(event EventHandleStartingNewPlayer
  (params (NewPlayer :type Player%20Controller%20Object%20Reference))
  (bind _returnvalue (Game|GetCurrentLevelName true))
  (switch string _returnvalue
    (:DuelMap
      (bind _asvrwestern_player_controller (Utilities|Casting|CastToVRWesternPlayerController NewPlayer))
      (CallFunction|AddPlayertoAllConnectedPlayers _asvrwestern_player_controller)
      (Utilities|FlowControl|DelayUntilNextTick)
      (Default|GameEntrySetup _asvrwestern_player_controller))))

(fn ConstructionScript)

(fn FindandFreePlayerStart
  (params (ExitingController :type Object%20Object%20Reference))
  (bind _occupiedplayerstarts (Variables|Default|GetOccupiedPlayerStarts))
  (bind _keys (Utilities|Map|Keys (Variables|Default|GetOccupiedPlayerStarts)))
  (bind _array_element (Utilities|Array|ForEachLoopwithBreak _keys :!label _label)
    (:LoopBody
      (if (== ExitingController (.Value (Utilities|Map|Find _occupiedplayerstarts _array_element)))
        (Utilities|Map|Remove _occupiedplayerstarts _array_element)
        (goto _label Break)))))

(fn AddPlayertoAllConnectedPlayers
  (params (NewPlayer :type VR%20Western%20Player%20Controller%20Object%20Reference))
  (bind _allconnectedplayers (Variables|Default|GetAllConnectedPlayers))
  (Utilities|Array|Add _allconnectedplayers NewPlayer)
  (if (== (Utilities|Array|Length _allconnectedplayers) 3)
    (CallFunction|AllPlayersConnected)))

(fn GetUnoccupiedPlayerStart
  (bind _outactors (Actor|GetAllActorsOfClass "/Script/Engine.PlayerStart"))
  (for _array_element _outactors
    (if (Utilities|Map|Contains (Variables|Default|GetOccupiedPlayerStarts) (Utilities|String|ToString(Name) (Variables|/Script/Engine.PlayerStart|GetPlayerStartTag _array_element)))
      (Utilities|Array|Add (LocalVariables|GetOccupiedPlayerStartArr) _array_element)
      (else
        (Utilities|Array|Add (LocalVariables|GetUnoccupiedPlayerStartArr) _array_element))))
  (return (LocalVariables|GetUnoccupiedPlayerStartArr) (LocalVariables|GetOccupiedPlayerStartArr)))

(fn TryGetHostPlayerStart
  (bind _as플레이어_스타트 (Utilities|Casting|CastToPlayerStart (Class|GameModeBase|FindPlayerStart (Game|GetPlayerController 0) "Host"))
    (:then
      (return _as플레이어_스타트 (== (Variables|/Script/Engine.PlayerStart|GetPlayerStartTag _as플레이어_스타트) "Host")))
    (:CastFailed
      (return 0 false))))