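; Actor that hosts a 2D on-screen keyboard widget and turns its button presses into simulated keyboard input.
; BeginPlay caches the Keyboard component's widget and collapses it.
; SetUpKeyboard rebinds the widget's button event and initializes its layout from a data table.
; On press, KeyPressed routes input through the WidgetInteraction component, sending characters for plain keys and key presses for Space, Backspace, Enter and arrows.
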(event Custom|KeyPressed
  (params (Text :type Text) (Pressed :type Boolean) (KeyType :type Keyboard%20Key%20Table%20Row%20Structure))
  (bind _widgetinteraction (Variables|Default|GetWidgetInteraction))
  (if Pressed
    (switch Utilities|FlowControl|Switch|SwitchonSpecialKeyType (.KeyEvent (Utilities|Struct|BreakKeyboardKeyTableRow KeyType))
      (:NewEnumerator10
        (Class|WidgetInteractionComponent|SendKeyChar (Variables|Default|GetWidgetInteraction) (Utilities|String|ToString(Text) Text) true))
      (:NewEnumerator4
        (Class|WidgetInteractionComponent|PressKey _widgetinteraction "SpaceBar" true))
      (:NewEnumerator5
        (Class|WidgetInteractionComponent|PressKey _widgetinteraction "BackSpace" true))
      (:NewEnumerator6
        (Class|WidgetInteractionComponent|PressKey _widgetinteraction "Enter" false))
      (:NewEnumerator16
        (Class|WidgetInteractionComponent|PressKey _widgetinteraction "Up" true))
      (:NewEnumerator17
        (Class|WidgetInteractionComponent|PressKey _widgetinteraction "Down" true))
      (:NewEnumerator18
        (Class|WidgetInteractionComponent|PressKey _widgetinteraction "Left" true))
      (:NewEnumerator19
        (Class|WidgetInteractionComponent|PressKey _widgetinteraction "Right" true)))))

(event Custom|SetUpKeyboard
  (bind _2dkeyboardwidget (Variables|Default|Get2DKeyboardWidget))
  (EventDispatchers|UnbindallEventsfromButtonEvent _2dkeyboardwidget)
  (EventDispatchers|BindEventtoButtonEvent _2dkeyboardwidget (delegate Custom|KeyPressed))
  (Default|InitKeyboard _2dkeyboardwidget "/Game/VRExp/Level/Keyboard/KeyboardDataTable.KeyboardDataTable"))

(event EventBeginPlay
  (bind _as2dkeyboard (Utilities|Casting|CastTo2DKeyboard (UserInterface|GetWidget (Variables|Default|GetKeyboard))))
  (bind _output_get (Variables|Default|Set2DKeyboardWidget _as2dkeyboard))
  (Widget|SetVisibility _output_get "Collapsed"))

(event Collision|EventActorBeginOverlap
  (params (OtherActor :type Actor%20Object%20Reference)))

(event EventTick
  (params (DeltaSeconds :type Float%20%28single-precision%29)))

(fn ConstructionScript)