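; Game mode for the VR main menu and lobby, tracking connected players, their ready states and occupied player starts.
; New controllers on the lobby map are registered and set up a tick later; logouts remove their entries and free their start.
; Ready changes rebroadcast the profile list, starting a ready sequence when exactly three players are all ready, or aborting it otherwise.
; Helpers find the Host start and sort others by tag occupancy.
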(event Custom|UpdateLobby
  (params (PlayerNames :type Boolean))
  (if PlayerNames
    (Utilities|Array|Clear (Variables|Default|GetAllPlayerProfiles))
    (for _array_element (Variables|Default|GetAllConnectedPlayers)
      (Utilities|Array|Add (Variables|Default|GetAllPlayerProfiles) (Variables|/Game/Blueprints/VRMainMenuPlayerController.VRMainMenuPlayerController_C|GetPlayerProfileInfo _array_element)))
    (Default|CallConnectedPlayerListChanged)))

(event Custom|PlayerReady
  (params (Player :type VR%20Main%20Menu%20Player%20Controller%20Object%20Reference) (IsReady :type Boolean))
  (Utilities|Array|SetArrayElem (Variables|Default|GetAllPlayersReadyStatus) (Utilities|Array|FindItem (Variables|Default|GetAllConnectedPlayers) Player) IsReady)
  (CallFunction|UpdateLobby true)
  (bind _isallready (CallFunction|CheckifAllReady))
  (if _isallready
    (Variables|Default|SetReadySequenceStarted true)
    (Default|CallStartReadySequence)
    (elif (Variables|Default|GetReadySequenceStarted)
      (Variables|Default|SetReadySequenceStarted false)
      (Default|CallAbortReadySequence))))

(event EventBeginPlay)

(event EventTick
  (params (DeltaSeconds :type Float%20%28single-precision%29)))

(event EventHandleStartingNewPlayer
  (params (NewPlayer :type Player%20Controller%20Object%20Reference))
  (bind _returnvalue (Game|GetCurrentLevelName true))
  (switch string _returnvalue
    (:LobbyMenuMap
      (bind _asvrmain_menu_player_controller (Utilities|Casting|CastToVRMainMenuPlayerController NewPlayer))
      (CallFunction|AddPlayertoAllConnectedPlayers _asvrmain_menu_player_controller)
      (Utilities|FlowControl|DelayUntilNextTick)
      (Default|LobbyEntrySetup _asvrmain_menu_player_controller))))

(event EventOnLogout
  (params (ExitingController :type Controller%20Object%20Reference))
  (bind _allconnectedplayers (Variables|Default|GetAllConnectedPlayers))
  (bind _asvrmain_menu_player_controller (Utilities|Casting|CastToVRMainMenuPlayerController ExitingController))
  (Utilities|Array|RemoveIndex (Variables|Default|GetAllPlayersReadyStatus) (Utilities|Array|FindItem _allconnectedplayers _asvrmain_menu_player_controller))
  (Utilities|Array|RemoveItem _allconnectedplayers _asvrmain_menu_player_controller)
  (CallFunction|UpdateLobby true)
  (CallFunction|FindandFreePlayerStart _asvrmain_menu_player_controller))

(event EventSetPlayerStartOccupied
  (params (OccupyingPlayer :type VR%20Western%20Player%20Controller%20Base%20Object%20Reference) (OccupyingPosition :type String))
  (bind _asvrmain_menu_player_controller (Utilities|Casting|CastToVRMainMenuPlayerController OccupyingPlayer))
  (Utilities|Map|Add (Variables|Default|GetOccupiedPlayerStarts) OccupyingPosition _asvrmain_menu_player_controller))

(fn ConstructionScript)

(fn AddPlayertoAllConnectedPlayers
  (params (NewPlayer :type VR%20Main%20Menu%20Player%20Controller%20Object%20Reference))
  (Utilities|Array|Add (Variables|Default|GetAllConnectedPlayers) NewPlayer)
  (Utilities|Array|Add (Variables|Default|GetAllPlayersReadyStatus) false))

(fn CheckifAllReady
  (if (== (Utilities|Array|Length (Variables|Default|GetAllPlayersReadyStatus)) 3)
    (for _array_element (Variables|Default|GetAllPlayersReadyStatus)
      (LocalVariables|SetbIsAllReady (and (LocalVariables|GetbIsAllReady) _array_element)))
    (return (LocalVariables|GetbIsAllReady))
    (else
      (return false))))

(fn FindandFreePlayerStart
  (params (ExitingController :type Object%20Object%20Reference))
  (bind _occupiedplayerstarts (Variables|Default|GetOccupiedPlayerStarts))
  (bind _keys (Utilities|Map|Keys (Variables|Default|GetOccupiedPlayerStarts)))
  (bind _array_element (Utilities|Array|ForEachLoopwithBreak _keys :!label _label)
    (:LoopBody
      (if (== ExitingController (.Value (Utilities|Map|Find _occupiedplayerstarts _array_element)))
        (Utilities|Map|Remove _occupiedplayerstarts _array_element)
        (goto _label Break)))))

(fn GetUnoccupiedPlayerStart
  (bind _outactors (Actor|GetAllActorsOfClass "/Script/Engine.PlayerStart"))
  (for _array_element _outactors
    (if (Utilities|Map|Contains (Variables|Default|GetOccupiedPlayerStarts) (Utilities|String|ToString(Name) (Variables|/Script/Engine.PlayerStart|GetPlayerStartTag _array_element)))
      (Utilities|Array|Add (LocalVariables|GetOccupiedPlayerStartArr) _array_element)
      (else
        (Utilities|Array|Add (LocalVariables|GetUnoccupiedPlayerStartArr) _array_element))))
  (return (LocalVariables|GetUnoccupiedPlayerStartArr) (LocalVariables|GetOccupiedPlayerStartArr)))

(fn TryGetHostPlayerStart
  (bind _as플레이어_스타트 (Utilities|Casting|CastToPlayerStart (Class|GameModeBase|FindPlayerStart (Game|GetPlayerController 0) "Host"))
    (:then
      (return _as플레이어_스타트 (== (Variables|/Script/Engine.PlayerStart|GetPlayerStartTag _as플레이어_스타트) "Host")))
    (:CastFailed
      (return 0 false))))