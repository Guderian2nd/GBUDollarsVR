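; Player controller for the VR main menu and lobby, supporting both headset and flat-screen players.
; HMD status routes main and multiplayer menus to a world MenuWidgetActor with keyboard or to the viewport, and likewise picks where the loading screen shows.
; Lobby entry loads or creates the saved profile and sends it to the game mode via server.
; Returning to menu destroys sessions, with the host ending clients' first.
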(event Custom|DisplayMPMenuUIToScreen
  (bind _self self)
  (Utilities|IsValid (Variables|Default|GetMultiplayer%20Menu)
    (:Is%20Valid
      _)
    (:Is%20Not%20Valid
      (bind _returnvalue (UserInterface|CreateWidget "/Game/Blueprints/UMGs/MultiplayerMenuWidget.MultiplayerMenuWidget_C" _self))
      (bind _output_get (Variables|Default|SetMultiplayer%20Menu _returnvalue))
      (EventDispatchers|BindEventtoBacktoMainMenu _output_get (delegate Custom|DisplayMainMenuUIToScreen))))
  (UserInterface|Viewport|AddtoViewport _output_get 0)
  (Input|SetInputModeUIOnly _self 0 "DoNotLock" false)
  (Variables|Default|SetbShowMouseCursor true))

(event Custom|DisplayMainMenuUIToScreen
  (bind _self self)
  (Utilities|IsValid (Variables|Default|GetMain%20Menu)
    (:Is%20Valid
      _)
    (:Is%20Not%20Valid
      (bind _returnvalue (UserInterface|CreateWidget "/Game/Blueprints/UMGs/MainMenuWidget.MainMenuWidget_C" _self))
      (bind _output_get (Variables|Default|SetMain%20Menu _returnvalue))
      (EventDispatchers|BindEventtoOpenMultiplayerMenu _output_get (delegate Custom|DisplayMPMenuUIToScreen))))
  (UserInterface|Viewport|AddtoViewport (Variables|Default|GetMain%20Menu) 0)
  (Input|SetInputModeUIOnly _self 0 "DoNotLock" false)
  (Variables|Default|SetbShowMouseCursor true))

(event Custom|EndClientSession
  (|DestroySession self
    (:then
      (Game|OpenLevel(byName) "MainMenuMap"))))

(event Custom|Server_UpdateLobby
  (params (NewPlayerProfile :type S%20Player%20Profile%20Structure))
  (Variables|Default|SetPlayerProfileInfo NewPlayerProfile)
  (bind _asvrmain_menu_game_mode (Utilities|Casting|CastToVRMainMenuGameMode (Game|GetGameMode)))
  (Default|UpdateLobby _asvrmain_menu_game_mode true))

(event Custom|LobbyEntrySetup
  (bind _saveprofile (CallFunction|LoadSaveProfile))
  (CallFunction|ServerUpdateLobby _saveprofile))

(event Custom|Return%20to%20Main%20Menu
  (if (Networking|IsServer)
    (bind _asvrmain_menu_game_mode (Utilities|Casting|CastToVRMainMenuGameMode (Game|GetGameMode)))
    (for _array_element (Variables|/Game/Blueprints/VRMainMenuGameMode.VRMainMenuGameMode_C|GetAllConnectedPlayers _asvrmain_menu_game_mode)
      (if (!= _array_element (Game|GetPlayerController 0))
        (CallFunction|EndClientSession _array_element)))
    (Utilities|FlowControl|Delay 0.3))
  (|DestroySession (Game|GetPlayerController 0)
    (:then
      (Game|OpenLevel(byName) "MainMenuMap"))))

(event Custom|CreateLoadingScreen
  (CallFunction|ShowLoadingScreenWdiget))

(event Custom|BindAndInitMainMenu
  (Utilities|IsValid (Variables|Default|GetMain%20Menu)
    (:Is%20Valid
      _)
    (:Is%20Not%20Valid
      (bind _returnvalue (UserInterface|CreateWidget "/Game/Blueprints/UMGs/MainMenuWidget.MainMenuWidget_C" self))
      (bind _output_get (Variables|Default|SetMain%20Menu _returnvalue))
      (EventDispatchers|BindEventtoOpenMultiplayerMenu _output_get (delegate Custom|BindAndInitMultiplayerMenu))))
  (bind _returnvalue_2 (Actor|GetActorOfClass "/Game/Blueprints/MenuWidgetActor.MenuWidgetActor_C"))
  (UserInterface|SetWidget (Variables|/Game/Blueprints/MenuWidgetActor.MenuWidgetActor_C|GetWidget _returnvalue_2) _output_get)
  (Default|SetUpKeyboard _returnvalue_2)
  (Widget|SetVisibility (Variables|/Game/Blueprints/MenuWidgetActor.MenuWidgetActor_C|Get2DKeyboardWidget _returnvalue_2) "Visible"))

(event Custom|BindAndInitMultiplayerMenu
  (Utilities|IsValid (Variables|Default|GetMultiplayer%20Menu)
    (:Is%20Valid
      _)
    (:Is%20Not%20Valid
      (bind _returnvalue (UserInterface|CreateWidget "/Game/Blueprints/UMGs/MultiplayerMenuWidget.MultiplayerMenuWidget_C" self))
      (bind _output_get (Variables|Default|SetMultiplayer%20Menu _returnvalue))
      (EventDispatchers|BindEventtoBacktoMainMenu _output_get (delegate Custom|BindAndInitMainMenu))))
  (bind _returnvalue_2 (Actor|GetActorOfClass "/Game/Blueprints/MenuWidgetActor.MenuWidgetActor_C"))
  (UserInterface|SetWidget (Variables|/Game/Blueprints/MenuWidgetActor.MenuWidgetActor_C|GetWidget _returnvalue_2) _output_get)
  (Widget|SetVisibility (Variables|/Game/Blueprints/MenuWidgetActor.MenuWidgetActor_C|Get2DKeyboardWidget _returnvalue_2) "Collapsed"))

(event Custom|ReturnToMainMenuServerCall
  (CallFunction|ReturntoMainMenu))

(event EventBeginPlay
  (|CallParentFunction) ; 지금 이 노드는 비활성 상태입니다. \n핀을 끌어서 다른 노드를 연결하면 활성화됩니다.
)

(event EventTick
  (params (DeltaSeconds :type Float%20%28single-precision%29)))

(event EventReturnHMDStatus
  (params (bHMDEnabled :type Boolean) (HMDOffset :type Vector :default "0, 0, 0") (HMDRotation :type Rotator :default "0, 0, 0"))
  (|CallParentFunction bHMDEnabled HMDOffset HMDRotation)
  (bind _returnvalue (Game|GetCurrentLevelName true))
  (switch string _returnvalue
    (:MainMenuMap
      (if bHMDEnabled
        (CallFunction|BindandInitMainMenu)
        (else
          (CallFunction|DisplayMainMenuUItoScreen))))))

(fn ConstructionScript
  (|CallParentFunction))

(fn LoadSaveProfile
  (bind _localslotname (Variables|Default|GetLocalSlotName))
  (bind _returnvalue (SaveGame|DoesSaveGameExist (Variables|Default|GetLocalSlotName)))
  (if _returnvalue
    _
    (else
      (bind _returnvalue_2 (SaveGame|CreateSaveGameObject "/Game/SavedData/SG_PlayerProfile.SG_PlayerProfile_C"))
      (SaveGame|SaveGametoSlot _returnvalue_2 _localslotname)))
  (bind _returnvalue_3 (SaveGame|LoadGamefromSlot _localslotname))
  (bind _assg_player_profile (Utilities|Casting|CastToSG_PlayerProfile _returnvalue_3))
  (bind _output_get (Variables|Default|SetPlayerProfileInfo (Variables|/Game/SavedData/SG_PlayerProfile.SG_PlayerProfile_C|GetPlayerProfile _assg_player_profile)))
  (Class|AdvancedSessionsLibrary|SetPlayerName self (Utilities|String|ToString(Text) (Utilities|Struct|BreakS_PlayerProfile _output_get)))
  (return _output_get))

(fn ShowLoadingScreenWdiget
  (bind _returnvalue (Pawn|GetControlledPawn))
  (if (Variables|Default|GetHMDEnabled)
    (Utilities|IsValid _returnvalue
      (:Is%20Valid
        (bind _newparam (Class|VRCharacterWidgetInterface|GetHMDWidgetComponent(Message) _returnvalue))
        (bind _returnvalue_2 (UserInterface|CreateWidget "/Game/Blueprints/UMGs/LoadingScreenWidget.LoadingScreenWidget_C" (Game|GetPlayerController 0)))
        (UserInterface|SetWidget _newparam _returnvalue_2)))
    (else
      (Viewport|RemoveAllWidgets)
      (Utilities|IsValid (Variables|Default|GetLoadingScreen)
        (:Is%20Valid
          _)
        (:Is%20Not%20Valid
          (bind _returnvalue_3 (UserInterface|CreateWidget "/Game/Blueprints/UMGs/LoadingScreenWidget.LoadingScreenWidget_C" self))
          (bind _output_get (Variables|Default|SetLoadingScreen _returnvalue_3))))
      (UserInterface|Viewport|AddtoViewport _output_get 0))))