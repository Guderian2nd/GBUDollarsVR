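; VR main-menu ready button that reports a player's ready state to VRMainMenuGameMode.
; On the server, button changes mark the interacting player ready or unready, signal ElectricalTargets and update the label text.
; RepServerButtonState reapplies the button state one tick after changes and whenever the connected-player list changes, apparently to sync clients.
; An incoming CurrentStateChange forces the button off on the server.
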(event OnButtonStateChanged(ButtonComp)
  (params (ButtonState :type Boolean) (InteractingActor :type Actor%20Object%20Reference) (InteractingComponent :type Primitive%20Component%20Object%20Reference))
  (bind _textrender (Variables|Default|GetTextRender))
  (if (Networking|IsServer)
    (bind _as폰 (Utilities|Casting|CastToPawn InteractingActor))
    (bind _asvrmain_menu_player_controller (Utilities|Casting|CastToVRMainMenuPlayerController (Pawn|GetController _as폰)))
    (bind _asvrmain_menu_game_mode (Utilities|Casting|CastToVRMainMenuGameMode (Game|GetGameMode)))
    (Default|PlayerReady _asvrmain_menu_game_mode _asvrmain_menu_player_controller ButtonState)
    ;[1 1 1] Send Out Electrical Signal
    (for _array_element (Variables|Default|GetElectricalTargets)
      (bind _aselectrical_object (Utilities|Casting|CastToElectricalObject _array_element))
      (Default|CurrentStateChange _aselectrical_object self ButtonState 1.0))
    (if ButtonState
      (Rendering|Components|TextRender|SetText _textrender (Variables|Default|GetOnText))
      (else
        (Rendering|Components|TextRender|SetText _textrender (Variables|Default|GetOffText))))
    (Utilities|FlowControl|DelayUntilNextTick)
    (CallFunction|RepServerButtonState ButtonState)))

(event Custom|RepServerButtonState
  (params (ButtonState :type Boolean))
  (Class|VRButtonComponent|SetButtonState (Variables|Default|GetButtonComp) ButtonState true true))

(event Custom|JoinedButtonSync
  (Utilities|FlowControl|DelayUntilNextTick)
  (CallFunction|RepServerButtonState (Variables|/Script/VRExpansionPlugin.VRButtonComponent|GetbButtonState (Variables|Default|GetButtonComp))))

(event EventBeginPlay
  (|CallParentFunction)
  (if (Networking|IsServer)
    (bind _asvrmain_menu_game_mode (Utilities|Casting|CastToVRMainMenuGameMode (Game|GetGameMode)))
    (EventDispatchers|BindEventtoConnectedPlayerListChanged _asvrmain_menu_game_mode (delegate Custom|JoinedButtonSync))))

(event Collision|EventActorBeginOverlap
  (params (OtherActor :type Actor%20Object%20Reference)))

(event EventTick
  (params (DeltaSeconds :type Float%20%28single-precision%29))
  (|CallParentFunction DeltaSeconds))

(event EventCurrentStateChange
  (params (CurrentProvider :type Object%20Object%20Reference) (ElectricalState :type Boolean) (CurrentFlow :type Float%20%28double-precision%29))
  (if (Networking|IsServer)
    (Class|VRButtonComponent|SetButtonState (Variables|Default|GetButtonComp) false true true)
    (CallFunction|RepServerButtonState false)))

(fn ConstructionScript
  (|CallParentFunction))