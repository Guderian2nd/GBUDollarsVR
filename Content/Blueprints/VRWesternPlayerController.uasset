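; Player controller for a VR western duel game, handling HUD setup, input modes and starting HP.
; Game entry retries each tick until a pawn exists, then puts the duel HUD on its HMD widget component, shows the player name and switches to UI-only input.
; Countdown sets HP on the authority, higher for Iron Man, and restores game-only input on remote.
; Events update HP text; death only prints a message.
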(event Custom|GameEntrySetup
  (bind _returnvalue (Pawn|GetControlledPawn))
  (Utilities|IsValid _returnvalue :!label _label
    (:Is%20Valid
      (bind _widgetcompofpawn (Class|VRCharacterWidgetInterface|GetHMDWidgetComponent(Message) _returnvalue))
      (bind _returnvalue_2 (UserInterface|CreateWidget "/Game/Blueprints/UMGs/WesternDuelHUD.WesternDuelHUD_C" self))
      (bind _output_get (Variables|Default|SetInGameHUD _returnvalue_2))
      (UserInterface|SetWidget _widgetcompofpawn _output_get)
      (bind _asbp_western_duel_player_state (Utilities|Casting|CastToBP_WesternDuelPlayerState (Variables|Default|GetPlayerState)))
      (Rendering|Components|TextRender|SetText (Variables|/Game/Blueprints/UMGs/WesternDuelHUD.WesternDuelHUD_C|GetPlayerNameText (Variables|Default|GetInGameHUD)) (Utilities|Struct|BreakS_PlayerProfile (Variables|/Game/Blueprints/BP_WesternDuelPlayerState.BP_WesternDuelPlayerState_C|GetS_PlayerProfile _asbp_western_duel_player_state)))
      (Input|SetInputModeUIOnly self (Variables|Default|GetInGameHUD) "DoNotLock" false))
    (:Is%20Not%20Valid
      (Utilities|FlowControl|DelayUntilNextTick)
      (goto _label))))

(event Custom|GameStartCountDown
  (params (IsIronMan :type Boolean))
  (bind _playerstate (Variables|Default|GetPlayerState))
  (Networking|SwitchHasAuthority
    (:Authority
      (if IsIronMan
        (bind _asbp_western_duel_player_state (Utilities|Casting|CastToBP_WesternDuelPlayerState _playerstate))
        (Variables|/Game/Blueprints/BP_WesternDuelPlayerState.BP_WesternDuelPlayerState_C|SetHP _asbp_western_duel_player_state 2)
        (else
          (bind _asbp_western_duel_player_state_2 (Utilities|Casting|CastToBP_WesternDuelPlayerState _playerstate))
          (Variables|/Game/Blueprints/BP_WesternDuelPlayerState.BP_WesternDuelPlayerState_C|SetHP _asbp_western_duel_player_state_2 1))))
    (:Remote
      (Input|SetInputModeGameOnly self false))))

(event Custom|UpdateWidgetHP
  (params (NewHPValue :type Integer))
  (bind _ingamehud (Variables|Default|GetInGameHUD))
  (Utilities|IsValid _ingamehud
    (:Is%20Valid
      (Rendering|Components|TextRender|SetText (Variables|/Game/Blueprints/UMGs/WesternDuelHUD.WesternDuelHUD_C|GetHPText _ingamehud) (Utilities|Text|ToText(String) (Utilities|String|Append "HP : " (Utilities|String|ToString(Integer) NewHPValue)))))))

(event Custom|HPIsZero
  (Development|PrintString "Dead!"))

(event EventBeginPlay
  (|CallParentFunction)
  (Input|SetInputModeGameOnly self false)
  (Variables|Default|SetbShowMouseCursor false)
  (Viewport|RemoveAllWidgets))

(event EventTick
  (params (DeltaSeconds :type Float%20%28single-precision%29)))

(fn ConstructionScript
  (|CallParentFunction))